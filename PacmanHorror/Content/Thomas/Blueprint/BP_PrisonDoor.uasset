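; BP_PrisonDoor is a prison door in a Pac-Man-style game that opens once red, blue and green keys are collected.
; On BeginPlay it shows a key tracker widget, then spawns the three key pieces at random pac-gums from BP_Pacman's list.
; Each spawn also destroys a randomly picked pac-gum, re-rolled separately from the spawn point.
; AddKey updates the HUD and flags; a full set triggers a timeline sliding both door meshes.
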(event `self.ReceiveBeginPlay`
  (bind _returnvalue (`|CreateWidget` "/Game/Thomas/Blueprint/WBP_KeyTracker.WBP_KeyTracker_C"))
  (bind _output_get (set `self.KeyRefHUD` _returnvalue))
  (`UserWidget.AddToViewport` _returnvalue 0)
  (`UserWidget.AddToViewport` _output_get 0)
  (`KismetSystemLibrary.Delay` 0.2)
  (bind _returnvalue_2 (`GameplayStatics.GetActorOfClass` "/Game/Blueprint/BP_Pacman.BP_Pacman_C"))
  (bind _output_get_2 (set `self.PacmanRef` _returnvalue_2))
  (bind _listpacgum (`/Game/Blueprint/BP_Pacman.ListPacGum` _output_get_2))
  (`self.SpawnKeyPiece` _listpacgum)
  (`self.SpawnKeyPiece` _listpacgum "NewEnumerator1")
  (`self.SpawnKeyPiece` _listpacgum "NewEnumerator2"))

(event `OpenPrisonDoor`
  (`TimelineComponent.SetPlayRate` (`self.DoorOpening`) (/ 1.0 3.0))
  (bind (_direction _newtrack_0) (`Timeline|DoorOpening`)
    (:`Update`
      (`SceneComponent.K2_SetRelativeLocation` (`self.StaticDoorMesh`) (`KismetMathLibrary.VLerp` (-100.0 0.0 0.0) (-200.0 0.0 0.0) _newtrack_0) false false)
      (`SceneComponent.K2_SetRelativeLocation` (`self.MovingDoorMesh`) (`KismetMathLibrary.VLerp` (0.0 0.0 0.0) (100.0 0.0 0.0) _newtrack_0) false false))))

(event `CheckForCOmpletion`
  (if (and (`self.HasRedKey?`) (and (`self.HasBlueKey?`) (`self.HasGreenKey?`)))
    (`self.OpenPrisonDoor`)))

(event `AddKey`
  (params (KeyType :type "/Game/Thomas/Blueprint/enum_KeyType Enum" :default "NewEnumerator0"))
  (`/Game/Thomas/Blueprint/WBP_KeyTracker.GetKey` (`self.KeyRefHUD`) KeyType)
  (switch `/Game/Thomas/Blueprint/enum_KeyType` KeyType
    (:`NewEnumerator0`
      (set `self.HasRedKey?` true))
    (:`NewEnumerator1`
      (set `self.HasBlueKey?` true))
    (:`NewEnumerator2`
      (set `self.HasGreenKey?` true)))
  (`self.CheckForCOmpletion`))

(fn `SpawnKeyPiece`
  (params (TargetArray :type "Array of /Game/Blueprint/BP_PacGum_Parent Object Reference (by ref)") (KeyType :type "/Game/Thomas/Blueprint/enum_KeyType Enum" :default "NewEnumerator0"))
  (bind _outitem (`KismetArrayLibrary.Array_Random` TargetArray))
  (`|SpawnActorFromClass` "/Game/Thomas/Blueprint/BP_KeyPiece.BP_KeyPiece_C" (`self.GetTransform` _outitem) "AlwaysSpawn" "MultiplyWithRoot" _outitem KeyType null)
  (`/Game/Blueprint/BP_PacGum_Parent.Destroy` _outitem (`self.PacmanRef`)))

(fn `UserConstructionScript`)