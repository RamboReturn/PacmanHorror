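; BP_KeyPiece is a colored key pickup that the player collects for the prison door.
; On BeginPlay it caches the BP_PrisonDoor found in the level and gives its mesh a red, blue or green glow material based on KeyType.
; When the player character overlaps the collision component, it passes KeyType to the door's AddKey, plays a pickup sound and destroys itself.
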(event `self.ReceiveBeginPlay`
  (bind _returnvalue (`GameplayStatics.GetActorOfClass` "/Game/Thomas/Blueprint/BP_PrisonDoor.BP_PrisonDoor_C"))
  (set `self.PrisonDoorRef` _returnvalue)
  (`PrimitiveComponent.SetMaterial` (`self.KeyMech`) 0 (select `/Game/Thomas/Blueprint/enum_KeyType` (`self.KeyType`) :`NewEnumerator0` "/Game/Thomas/Materials/MI_RedGlow.MI_RedGlow" :`NewEnumerator1` "/Game/Thomas/Materials/MI_BlueGlow.MI_BlueGlow" :`NewEnumerator2` "/Game/Thomas/Materials/MI_GreenGlow.MI_GreenGlow" :!type "MaterialInterface Object Reference")))

(event `self.PlayerCollision.OnComponentBeginOverlap`
  (params (OverlappedComponent :type "PrimitiveComponent Object Reference") (OtherActor :type "Actor Object Reference") (OtherComp :type "PrimitiveComponent Object Reference") (OtherBodyIndex :type Integer) (bFromSweep :type Boolean) (SweepResult :type "HitResult Structure (by ref)"))
  (if (== OtherActor (`GameplayStatics.GetPlayerCharacter` 0))
    (`/Game/Thomas/Blueprint/BP_PrisonDoor.AddKey` (`self.PrisonDoorRef`) (`self.KeyType`))
    (`GameplayStatics.PlaySoundAtLocation` (`self.PickUpSound`) (`self.K2_GetActorLocation`) (struct) 1.0 1.0 0.0 null null null null)
    (`self.K2_DestroyActor`)))

(fn `UserConstructionScript`)