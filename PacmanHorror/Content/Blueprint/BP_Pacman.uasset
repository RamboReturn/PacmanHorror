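; BP_Pacman is an AI enemy that hunts pac-gums and the player, triggering game over when its box overlaps the player.
; It moves to random pac-gums and eats them, chasing the player permanently if the list is empty.
; Pawn sensing starts a chase with aggro audio, which a retriggerable delay ends while gums remain.
; BigPacGunEffect temporarily boosts walk speed and animation rate through a timeline.
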(event `self.ReceiveBeginPlay`
  (bind _outactors (`GameplayStatics.GetAllActorsOfClass` "/Game/Blueprint/BP_PacGum_Parent.BP_PacGum_Parent_C"))
  (set `self.ListPacGum` _outactors)
  (set `CharacterMovementComponent.MaxWalkSpeed` (`self.Speed`) (`self.CharacterMovement`))
  (bind _returnvalue (`GameplayStatics.GetActorOfClass` "/Game/ThirdPerson/Blueprints/BP_ThirdPersonCharacter.BP_ThirdPersonCharacter_C"))
  (set `self.Player` _returnvalue)
  (`self.GetPacGum`)
  (bind _returnvalue_2 (`GameplayStatics.SpawnSoundAttached` "/Game/Thomas/Sound/PacAmb_Cue.PacAmb_Cue" (`self.CapsuleComponent`) "None" (0.0 0.0 0.0) (struct) "KeepRelativeOffset" false 1.0 1.0 0.0 null null))
  (set `self.PAcAmbSound` _returnvalue_2))

(event `StartMovement`
  (bind _player (`self.Player`))
  (bind _activepacgum (`self.ActivePacGum`))
  (if (`self.ChasePlayer`)
    (`|AIMoveTo` self (`self.K2_GetActorLocation` _player) _player 5.0 true)
    (else
      (`|AIMoveTo` self (`self.K2_GetActorLocation` _activepacgum) _activepacgum 0.5
        (:`OnSuccess`
          (`self.DelActivePacGum`))))))

(event `GetPacGum`
  (bind (_outitem _outindex) (`KismetArrayLibrary.Array_Random` (`self.ListPacGum`)))
  (if (> (`KismetArrayLibrary.Array_Length` (`self.ListPacGum`)) 0)
    (set `self.ActivePacGum` _outitem)
    (set `self.Index` _outindex)
    (else
      (set `self.ChasePlayer` true)))
  (`self.StartMovement`))

(event `self.ReceiveActorBeginOverlap`
  (params (OtherActor :type "Actor Object Reference"))
  (if (!= OtherActor (`self.ActivePacGum`))
    (bind _asbp_pac_gum_parent (cast `/Game/Blueprint/BP_PacGum_Parent` OtherActor)
      (:`then`
        (`/Game/Blueprint/BP_PacGum_Parent.Destroy` _asbp_pac_gum_parent self))
      (:`CastFailed`
        (bind _asbp_third_person_character (cast `/Game/ThirdPerson/Blueprints/BP_ThirdPersonCharacter` OtherActor))))))

(event `DelActivePacGum`
  (`/Game/Blueprint/BP_PacGum_Parent.Destroy` (`self.ActivePacGum`) self)
  (`self.GetPacGum`))

(event `BigPacGunEffect`
  (bind _skeletalmesh (`self.SkeletalMesh`))
  (set `CharacterMovementComponent.MaxWalkSpeed` (`self.BoostSpeed`) (`self.CharacterMovement`))
  (`SkeletalMeshComponent.SetPlayRate` _skeletalmesh 4.0)
  (`Timeline|Boost` :!via `PlayFromStart`
    (:`Finished`
      (set `CharacterMovementComponent.MaxWalkSpeed` (`self.Speed`) (`self.CharacterMovement`))
      (`SkeletalMeshComponent.SetPlayRate` _skeletalmesh 1.0))))

(event `self.PawnSensing.OnSeePawn`
  (params (Pawn :type "Pawn Object Reference"))
  (`|ExecutionSequence`
    (:`then_0`
      (`KismetSystemLibrary.PrintString` "Player seen")
      (set `self.ChasePlayer` true)
      (`self.StartMovement`)
      (`KismetSystemLibrary.RetriggerableDelay` 5.0)
      (if (> (`KismetArrayLibrary.Array_Length` (`self.ListPacGum`)) 0)
        (set `self.ChasePlayer` false)
        (`KismetSystemLibrary.PrintString` "lost player")
        (`self.StartMovement`)
        (`AudioComponent.Stop` (`self.AggroSound`))
        (`AudioComponent.Play` (`self.PAcAmbSound`) 0.0)
        (goto _label :!via `Reset`)))
    (:`then_1`
      (`/Engine/EditorBlueprintResources/StandardMacros.DoOnce` false :!label _label
        (:`Completed`
          (`AudioComponent.Stop` (`self.PAcAmbSound`))
          (bind _returnvalue (`GameplayStatics.SpawnSoundAttached` "/Game/Thomas/Sound/PAcAgro.PAcAgro" (`self.CapsuleComponent`) "None" (0.0 0.0 0.0) (struct) "KeepRelativeOffset" false 1.0 1.0 0.0 null null))
          (set `self.AggroSound` _returnvalue))))))

(event `self.Box.OnComponentBeginOverlap`
  (params (OverlappedComponent :type "PrimitiveComponent Object Reference") (OtherActor :type "Actor Object Reference") (OtherComp :type "PrimitiveComponent Object Reference") (OtherBodyIndex :type Integer) (bFromSweep :type Boolean) (SweepResult :type "HitResult Structure (by ref)"))
  (bind _player (`self.Player`))
  (if (== OtherActor _player)
    (`/Game/ThirdPerson/Blueprints/BP_ThirdPersonCharacter.GameOver` _player)))

(fn `UserConstructionScript`)